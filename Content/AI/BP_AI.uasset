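; Demon enemy character that spots and claws the player, with health and a death sequence.
; Pawn sensing sets the seeingPlayer blackboard key, cleared by a looping timer, and triggers a one-time, player-gated alert sound.
; AttackPlayer plays a slash montage and immediately sphere-traces forward to apply damage, blocking re-entry until the montage completes.
; Incoming damage lowers health; at zero, the demon plays a death montage, stops moving and is destroyed after a delay.
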(event `self.ReceiveBeginPlay`
  (`KismetSystemLibrary.K2_SetTimerDelegate` (delegate `Stop Seeing Player`) 0.8 true)
  (bind _returnvalue (`AddComponent|NODE_AddAudioComponent-1`))
  (`AudioComponent.Stop` _returnvalue)
  (set `self.SeePlayerAudio` _returnvalue)
  (set `self.Health` 100.0))

(event `Stop Seeing Player`
  (`BlackboardComponent.SetValueAsBool` (`AIBlueprintHelperLibrary.GetBlackboard` (`AIBlueprintHelperLibrary.GetAIController` self)) "seeingPlayer" false))

(event `self.PawnSensing.OnSeePawn`
  (params (Pawn :type "Pawn Object Reference"))
  ;[1 0.5687 0.6836] See Player
  (if (`self.ActorHasTag` Pawn "Player")
    (`BlackboardComponent.SetValueAsBool` (`AIBlueprintHelperLibrary.GetBlackboard` (`AIBlueprintHelperLibrary.GetAIController` self)) "seeingPlayer" true)
    (`/Engine/EditorBlueprintResources/StandardMacros.DoOnce` false
      (:`Completed`
        (bind _asfirst_person_character_new (cast `/Game/HUahhah/FirstPersonBP/Blueprints/FirstPersonCharacterNew` (`GameplayStatics.GetPlayerCharacter` 0)))
        (if (`/Game/HUahhah/FirstPersonBP/Blueprints/FirstPersonCharacterNew.SoundPlay` _asfirst_person_character_new)
          (`AudioComponent.Play` (`self.SeePlayerAudio`) 0.0)
          (bind _asfirst_person_character_new_2 (cast `/Game/HUahhah/FirstPersonBP/Blueprints/FirstPersonCharacterNew` (`GameplayStatics.GetPlayerCharacter` 0)))
          (`/Game/HUahhah/FirstPersonBP/Blueprints/FirstPersonCharacterNew.SeeSound` _asfirst_person_character_new_2))))))

(event `Attack Player`
  (bind _attack_trace_point (`self.Attack Trace Point`))
  (bind _returnvalue (`SceneComponent.K2_GetComponentLocation` _attack_trace_point))
  ;[1 0.9256 0.1935] Attack Player
  (if (not (`self.attacking`))
    (set `self.attacking` true)
    (`|PlayMontage` (`self.Mesh`) "/Game/AI/Demon_Anim_metarig_SlashFromSideForward_Montage.Demon_Anim_metarig_SlashFromSideForward_Montage"
      (:`then`
        (bind (_outhit _returnvalue_2) (`KismetSystemLibrary.SphereTraceSingleForObjects` _returnvalue (+ _returnvalue (* (`KismetMathLibrary.GetForwardVector` (`SceneComponent.K2_GetComponentRotation` _attack_trace_point)) 70.0)) 25.0 (`|MakeArray` "ObjectTypeQuery3" :!type "EObjectTypeQuery Enum")))
        (if _returnvalue_2
          (`GameplayStatics.ApplyDamage` (`.HitActor` (`GameplayStatics.BreakHitResult` _outhit)) 10.0)
          (`GameplayStatics.PlaySound2D` "/Game/AI/Audio/Claw_Attack.Claw_Attack" 1.0 1.0 0.0 null null)
          (`GameplayStatics.PlaySound2D` "/Game/AI/Audio/Blood_Splatter.Blood_Splatter" 1.0 1.0 0.0 null null)))
      (:`OnCompleted`
        (set `self.attacking` false)))))

(event `self.ReceiveAnyDamage`
  (params (Damage :type "Float (single-precision)") (DamageType :type "DamageType Object Reference") (InstigatedBy :type "Controller Object Reference") (DamageCauser :type "Actor Object Reference"))
  ;[1 1 1] Take DMG
  (if (not (`self.bDeath`))
    (bind _output_get (set `self.Health` (- (`self.Health`) Damage)))
    (`KismetSystemLibrary.PrintString` (`KismetStringLibrary.Conv_DoubleToString` _output_get))
    (if (<= _output_get 0.0)
      (`self.Death`))))

(event `Death`
  ;[1 1 1] Death
  (set `self.bDeath` true)
  (`GameplayStatics.PlaySound2D` "/Game/AI/Audio/Death/MonsterDeath.MonsterDeath" 1.0 1.0 0.0 null null)
  (`|PlayMontage` (`self.Mesh`) "/Game/AI/Demon_Anim_metarig_DizzyIdle_Montage.Demon_Anim_metarig_DizzyIdle_Montage"
    (:`then`
      (`CharacterMovementComponent.DisableMovement` (`self.CharacterMovement`))
      (`KismetSystemLibrary.Delay` 4.0)
      (`self.K2_DestroyActor`))))

(fn `UserConstructionScript`)