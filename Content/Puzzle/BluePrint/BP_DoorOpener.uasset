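; A puzzle door opener actor that opens a door once enough items have been collected.
; CollectItem increments a counter, and OpenDoorCheck compares it to the maximum, calling OpenDoor through a DoOnce so the door opens only once.
; Overlapping the Trigger component shows a widget, and leaving it hides the widget again.
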(event `Collect Item`
  (`/Engine/EditorBlueprintResources/StandardMacros.IncrementInt` (`self.currentItemCollected`)))

(event `Open Door Check`
  (if (>= (`self.currentItemCollected`) (`self.maxItemCollectable`))
    (`/Engine/EditorBlueprintResources/StandardMacros.DoOnce` false
      (:`Completed`
        (`self.OpenDoor`)))))

(event `self.Trigger.OnComponentBeginOverlap`
  (params (OverlappedComponent :type "PrimitiveComponent Object Reference") (OtherActor :type "Actor Object Reference") (OtherComp :type "PrimitiveComponent Object Reference") (OtherBodyIndex :type Integer) (bFromSweep :type Boolean) (SweepResult :type "HitResult Structure (by ref)"))
  (`SceneComponent.SetVisibility` (`self.Widget`) true false))

(event `self.Trigger.OnComponentEndOverlap`
  (params (OverlappedComponent :type "PrimitiveComponent Object Reference") (OtherActor :type "Actor Object Reference") (OtherComp :type "PrimitiveComponent Object Reference") (OtherBodyIndex :type Integer))
  (`SceneComponent.SetVisibility` (`self.Widget`) false false))

(fn `UserConstructionScript`)